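; Player character Blueprint child that, on BeginPlay, caches its ABP_BaseCharacter anim instance and PlayerController, then adds Enhanced Input contexts for movement, mouse and view.
; Tick only calls the parent, and the jump and view input events are empty.
; Logic for camera and head rotation, first/third-person switching and zoom, anim move-state updates, and a jump step-height boost remains in the graph but is disconnected and never runs.
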(event Input|EnhancedActionEvents|EnhancedInputActionINPA_Move
  (params (ActionValue :type Vector%202D%20Structure) (ElapsedSeconds :type Float%20%28double-precision%29) (TriggeredSeconds :type Float%20%28double-precision%29) (InputAction :type Input%20Action%20Object%20Reference :default "/Game/Main/Inputs/INPA_Move.INPA_Move"))
  ;[1 1 1] Инпут передвижения
)

(event Input|EnhancedActionEvents|EnhancedInputActionINPA_Jump
  (params (ActionValue :type Boolean) (ElapsedSeconds :type Float%20%28double-precision%29) (TriggeredSeconds :type Float%20%28double-precision%29) (InputAction :type Input%20Action%20Object%20Reference :default "/Game/Main/Inputs/INPA_Jump.INPA_Jump"))
  ;[1 1 1] Инпут передвижения
)

(event Input|EnhancedActionEvents|EnhancedInputActionINPA_ViewChange
  (params (ActionValue :type Boolean) (ElapsedSeconds :type Float%20%28double-precision%29) (TriggeredSeconds :type Float%20%28double-precision%29) (InputAction :type Input%20Action%20Object%20Reference :default "/Game/Main/Inputs/INPA_ViewChange.INPA_ViewChange"))
  ;[1 1 1] Инпут передвижения
)

(event Input|EnhancedActionEvents|EnhancedInputActionINPA_View3PRegulate
  (params (ActionValue :type Float%20%28double-precision%29) (ElapsedSeconds :type Float%20%28double-precision%29) (TriggeredSeconds :type Float%20%28double-precision%29) (InputAction :type Input%20Action%20Object%20Reference :default "/Game/Main/Inputs/INPA_View3PRegulate.INPA_View3PRegulate"))
  ;[1 1 1] Инпут передвижения
)

(event EventTick
  (params (DeltaSeconds :type Float%20%28single-precision%29))
  (|CallParentFunction DeltaSeconds))

(event EventBeginPlay
  (|CallParentFunction)
  (CallFunction|InitialVaribles))

(fn ConstructionScript)

(fn InitialVaribles
  (Utilities|FlowControl|Sequence
    (:then_0
      (bind _asabp_base_character (Utilities|Casting|CastToABP_BaseCharacter (Components|SkeletalMesh|GetAnimInstance (Variables|Character|GetMesh))))
      (Variables|Other|SetPlayerABP _asabp_base_character))
    (:then_1
      (bind _asplayer_controller (Utilities|Casting|CastToPlayerController (Pawn|GetController)))
      (bind _output_get (Variables|Other|SetPlayerController _asplayer_controller))
      (Utilities|IsValid (PlayerController|LocalPlayerSubsystems|GetEnhancedInputLocalPlayerSubsystem _output_get)
        (:Is%20Valid
          (Input|AddMappingContext (PlayerController|LocalPlayerSubsystems|GetEnhancedInputLocalPlayerSubsystem (Variables|Other|GetPlayerController)) "/Game/Main/Inputs/INPC_Move.INPC_Move" 0 "(bIgnoreAllPressedKeysUntilRelease=True,bForceImmediately=False,bNotifyUserSettings=False)")
          (Input|AddMappingContext (PlayerController|LocalPlayerSubsystems|GetEnhancedInputLocalPlayerSubsystem (Variables|Other|GetPlayerController)) "/Game/Main/Inputs/INPC_Mouse.INPC_Mouse" 0 "(bIgnoreAllPressedKeysUntilRelease=True,bForceImmediately=False,bNotifyUserSettings=False)")
          (Input|AddMappingContext (PlayerController|LocalPlayerSubsystems|GetEnhancedInputLocalPlayerSubsystem (Variables|Other|GetPlayerController)) "/Game/Main/Inputs/INPC_View.INPC_View" 0 "(bIgnoreAllPressedKeysUntilRelease=True,bForceImmediately=False,bNotifyUserSettings=False)"))))))