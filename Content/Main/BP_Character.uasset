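; Player character Blueprint with Enhanced Input movement, jumping and switchable first/third-person camera.
; Each tick rotates the camera with clamps that tighten horizontally while moving, and feeds head look-at and Stay/Move/Fall state to ABP_BaseCharacter.
; Move input sends a direction vector to the AnimBP, using a WichExec macro to zero it on release and a run input to scale it.
; View regulation adjusts third-person distance and switches views at the limit.
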(event Input|EnhancedActionEvents|EnhancedInputActionINPA_Move
  (params (ActionValue :type Vector%202D%20Structure) (ElapsedSeconds :type Float%20%28double-precision%29) (TriggeredSeconds :type Float%20%28double-precision%29) (InputAction :type Input%20Action%20Object%20Reference :default "/Game/Main/INPA_Move.INPA_Move"))
  ;[1 1 1] Инпут передвижения
  (:Triggered
    (if (AI|Components|NavMovement|IsMovingonGround (Variables|Character|GetCharacterMovement))
      (bind _isa (Utilities|WichExec :!label _label)
        (:Exec
          (bind _returnvalue (Class|CPPBaseCharacter|CalculateMovementDirection (Math|Vector2D|Normalize2D ActionValue) (Math|Float|SelectFloat (Math|Float|SelectFloat 1.0 0.5 (Input|EnhancedActionValues|GetINPA_MoveRun)) 0.0 _isa)))
          (Utilities|FlowControl|Sequence
            (:then_0
              (bind _playerabp (Variables|Other|GetPlayerABP)
                (:then
                  (Variables|/EntityAnimations/Human/ABP_BaseCharacter.ABP_BaseCharacter_C|SetMoveVector _playerabp _returnvalue))
                (:else))))))))
  (:Canceled
    (goto _label B))
  (:Completed
    (goto _label B)))

(event Input|EnhancedActionEvents|EnhancedInputActionINPA_Jump
  (params (ActionValue :type Boolean) (ElapsedSeconds :type Float%20%28double-precision%29) (TriggeredSeconds :type Float%20%28double-precision%29) (InputAction :type Input%20Action%20Object%20Reference :default "/Game/Main/INPA_Jump.INPA_Jump"))
  ;[1 1 1] Инпут передвижения
  (Character|Jump))

(event Input|EnhancedActionEvents|EnhancedInputActionINPA_ViewChange
  (params (ActionValue :type Boolean) (ElapsedSeconds :type Float%20%28double-precision%29) (TriggeredSeconds :type Float%20%28double-precision%29) (InputAction :type Input%20Action%20Object%20Reference :default "/Game/Main/INPA_ViewChange.INPA_ViewChange"))
  ;[1 1 1] Инпут передвижения
  (:Started
    (Class|CPPBaseCharacter|ChangeCameraView (not (Variables|Default|GetisThridView)) false)))

(event Input|EnhancedActionEvents|EnhancedInputActionINPA_View3PRegulate
  (params (ActionValue :type Float%20%28double-precision%29) (ElapsedSeconds :type Float%20%28double-precision%29) (TriggeredSeconds :type Float%20%28double-precision%29) (InputAction :type Input%20Action%20Object%20Reference :default "/Game/Main/INPA_View3PRegulate.INPA_View3PRegulate"))
  ;[1 1 1] Инпут передвижения
  (Class|CPPBaseCharacter|ChangeThridCameraDistance (* ActionValue 0.05))
  (if (or (and (> ActionValue 0.0) (not (Variables|Default|GetisThridView))) (Math|Boolean|ANDBoolean (< ActionValue 0.0) (Variables|Default|GetisThridView) (Math|Float|NearlyEqual(Float) (Variables|Default|GetcurrentThridPersonDistance) 0.0 1e-06)))
    (Class|CPPBaseCharacter|ChangeCameraView (not (Variables|Default|GetisThridView)) false)))

(event EventTick
  (params (DeltaSeconds :type Float%20%28single-precision%29))
  (bind _movevector (Variables|Default|GetMoveVector))
  (bind _returnvalue (Math|Vector2D|Vector2DLength _movevector))
  (bind _returnvalue_2 (Math|Vector2D|Vector2DLength _movevector))
  (bind _returnvalue_3 (Math|Float|Lerp 75.0 75.0 _returnvalue))
  (bind _returnvalue_4 (Math|Float|Lerp 5e+01 15.0 _returnvalue_2))
  (|CallParentFunction DeltaSeconds)
  (bind _playerabp (Variables|Other|GetPlayerABP)
    (:then
      (Variables|/EntityAnimations/Human/ABP_BaseCharacter.ABP_BaseCharacter_C|SetMoveState _playerabp (Variables|Default|GetMoveState))
      (Class|CPPBaseCharacter|EqualizationControllertoCamera 5.0 3.0 DeltaSeconds 2.0 (Variables|Other|GetPlayerController))
      (bind _returnvalue_5 (Class|CPPBaseCharacter|CalculateHeadRotation "(X=-55.000000,Y=55.000000)"))
      (bind _playerabp_2 (Variables|Other|GetPlayerABP)
        (:then
          (Variables|/EntityAnimations/Human/ABP_BaseCharacter.ABP_BaseCharacter_C|SetLook%20At%20Location _playerabp_2 _returnvalue_5)
          (Class|CPPBaseCharacter|RotateCamera (Math|Vector2D|MakeVector2D (* _returnvalue_4 -1.0) _returnvalue_4) (Math|Vector2D|MakeVector2D (* _returnvalue_3 -1.0) _returnvalue_3) (Input|EnhancedActionValues|GetINPA_Mouse) 2.0 (Variables|Other|GetPlayerController))
          (if (AI|Components|NavMovement|IsMovingonGround (Variables|Character|GetCharacterMovement))
            (Variables|Default|SetMoveState (select (Math|Float|NearlyEqual(Float) (Math|Vector2D|Vector2DLength (Variables|Default|GetMoveVector)) 0.0 1e-06) "Stay" "Move"))
            (else
              (Variables|Default|SetMoveState "Fall")
              (Class|CPPBaseCharacter|CalculateMovementDirection))))
        (:else)))
    (:else)))

(event EventBeginPlay
  (|CallParentFunction)
  (CallFunction|InitialVaribles))

(fn ConstructionScript)

(fn InitialVaribles
  (Utilities|FlowControl|Sequence
    (:then_0
      (bind _asabp_base_character (Utilities|Casting|CastToABP_BaseCharacter (Components|SkeletalMesh|GetAnimInstance (Variables|Character|GetMesh))))
      (Variables|Other|SetPlayerABP _asabp_base_character))
    (:then_1
      (bind _asplayer_controller (Utilities|Casting|CastToPlayerController (Pawn|GetController)))
      (bind _output_get (Variables|Other|SetPlayerController _asplayer_controller))
      (Utilities|IsValid (PlayerController|LocalPlayerSubsystems|GetEnhancedInputLocalPlayerSubsystem _output_get)
        (:Is%20Valid
          (Input|AddMappingContext (PlayerController|LocalPlayerSubsystems|GetEnhancedInputLocalPlayerSubsystem (Variables|Other|GetPlayerController)) "/Game/Main/INPC_Move.INPC_Move" 0 "(bIgnoreAllPressedKeysUntilRelease=True,bForceImmediately=False,bNotifyUserSettings=False)")
          (Input|AddMappingContext (PlayerController|LocalPlayerSubsystems|GetEnhancedInputLocalPlayerSubsystem (Variables|Other|GetPlayerController)) "/Game/Main/INPC_Mouse.INPC_Mouse" 0 "(bIgnoreAllPressedKeysUntilRelease=True,bForceImmediately=False,bNotifyUserSettings=False)")
          (Input|AddMappingContext (PlayerController|LocalPlayerSubsystems|GetEnhancedInputLocalPlayerSubsystem (Variables|Other|GetPlayerController)) "/Game/Main/INPC_View.INPC_View" 0 "(bIgnoreAllPressedKeysUntilRelease=True,bForceImmediately=False,bNotifyUserSettings=False)"))))))