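; BP_BasicHUD is a base-style HUD Blueprint that creates and displays the UI_HudBase widget.
; On BeginPlay it creates the widget if none is valid, assigns it to its Widget component, and adds that component's widget to the player screen.
; It calls an empty BindingEvents function before display and CallOnHudInit afterwards, and exposes the widget through GetHUD.
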(event EventBeginPlay
  (|CallParentFunction)
  (CallFunction|InitVariables)
  (CallFunction|BindingEvents)
  (UserInterface|Viewport|AddtoPlayerScreen (UserInterface|GetUserWidgetObject (Variables|Default|GetWidget)) 1)
  (Default|CallOnHudInit))

(event Collision|EventActorBeginOverlap
  (params (OtherActor :type Actor%20Object%20Reference)))

(event EventTick
  (params (DeltaSeconds :type Float%20%28single-precision%29)))

(fn ConstructionScript)

(fn InitVariables
  (Variables|Default|GetHud
    (:then)
    (:else
      (bind _returnvalue (UserInterface|CreateWidget "/Game/Main/Blueprints/UI/UI_HudBase.UI_HudBase_C"))
      (bind _output_get (Variables|Default|SetHud _returnvalue))
      (UserInterface|SetWidget (Variables|Default|GetWidget) _output_get))))

(fn BindingEvents)

(fn GetHUD
  (return (Variables|Default|GetHud)))