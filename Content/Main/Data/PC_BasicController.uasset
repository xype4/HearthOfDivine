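; Basic player controller that routes Enhanced Input for movement, jump, camera and interaction to the playable pawn and manages fullscreen widgets.
; Once the HUD initializes, it opens the player HUD and tracks opened widgets in an array, toggling menus by class.
; Active widgets show the cursor and remove gameplay mapping contexts until all are closed, leaving the menu context.
; Escape-menu input closes the last active widget, otherwise toggles the pause menu.
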(event Input|EnhancedActionEvents|EnhancedInputActionINPA_Move
  (params (ActionValue :type Vector%202D%20Structure) (ElapsedSeconds :type Float%20%28double-precision%29) (TriggeredSeconds :type Float%20%28double-precision%29) (InputAction :type Input%20Action%20Object%20Reference :default "/Game/Main/Inputs/INPA_Move.INPA_Move"))
  ;[1 1 1] Инпуты павна
  (:Triggered
    (bind _isa (Utilities|WichExec :!label _label)
      (:Exec
        (bind _playerpawn (Variables|Other|GetPlayerPawn)
          (:then
            (Class|CPPBaseCharacter|MovementInput _playerpawn ActionValue (Math|Float|SelectFloat (Math|Float|SelectFloat 1.0 0.5 (Input|EnhancedActionValues|GetINPA_MoveRun)) 0.0 _isa)))
          (:else)))))
  (:Canceled
    (goto _label B))
  (:Completed
    (goto _label B)))

(event Input|EnhancedActionEvents|EnhancedInputActionINPA_Jump
  (params (ActionValue :type Boolean) (ElapsedSeconds :type Float%20%28double-precision%29) (TriggeredSeconds :type Float%20%28double-precision%29) (InputAction :type Input%20Action%20Object%20Reference :default "/Game/Main/Inputs/INPA_Jump.INPA_Jump"))
  ;[1 1 1] Инпуты павна
  (bind _playerpawn (Variables|Other|GetPlayerPawn)
    (:then
      (Class|CPPBaseCharacter|JumpInput _playerpawn))
    (:else)))

(event Input|EnhancedActionEvents|EnhancedInputActionINPA_ViewChange
  (params (ActionValue :type Boolean) (ElapsedSeconds :type Float%20%28double-precision%29) (TriggeredSeconds :type Float%20%28double-precision%29) (InputAction :type Input%20Action%20Object%20Reference :default "/Game/Main/Inputs/INPA_ViewChange.INPA_ViewChange"))
  ;[1 1 1] Инпуты павна
  (bind _playerpawn (Variables|Other|GetPlayerPawn)
    (:then
      (Class|CPPBaseCharacter|ChangeCameraView (Variables|Other|GetPlayerPawn) (not (Variables|/Script/EntityClasses.CPP_BaseCharacter|GetisThridView _playerpawn)) false))
    (:else)))

(event Input|EnhancedActionEvents|EnhancedInputActionINPA_View3PRegulate
  (params (ActionValue :type Float%20%28double-precision%29) (ElapsedSeconds :type Float%20%28double-precision%29) (TriggeredSeconds :type Float%20%28double-precision%29) (InputAction :type Input%20Action%20Object%20Reference :default "/Game/Main/Inputs/INPA_View3PRegulate.INPA_View3PRegulate"))
  ;[1 1 1] Инпуты павна
  (bind _playerpawn (Variables|Other|GetPlayerPawn)
    (:then
      (Class|CPPBaseCharacter|ChangeThridCameraDistance _playerpawn ActionValue))
    (:else)))

(event Input|EnhancedActionEvents|EnhancedInputActionINPA_Mouse
  (params (ActionValue :type Vector%202D%20Structure) (ElapsedSeconds :type Float%20%28double-precision%29) (TriggeredSeconds :type Float%20%28double-precision%29) (InputAction :type Input%20Action%20Object%20Reference :default "/Game/Main/Inputs/INPA_Mouse.INPA_Mouse"))
  ;[1 1 1] Инпуты павна
  (:Triggered
    (bind _playerpawn (Variables|Other|GetPlayerPawn :!label _label)
      (:then
        (Class|CPPBaseCharacter|MouseInput _playerpawn ActionValue))
      (:else)))
  (:Canceled
    (goto _label))
  (:Completed
    (goto _label)))

(event Input|EnhancedActionEvents|EnhancedInputActionINPA_ExitAndMenu
  (params (ActionValue :type Boolean) (ElapsedSeconds :type Float%20%28double-precision%29) (TriggeredSeconds :type Float%20%28double-precision%29) (InputAction :type Input%20Action%20Object%20Reference :default "/Game/Main/Inputs/INPA_ExitAndMenu.INPA_ExitAndMenu"))
  ;[1 1 1] Инпуты меню
  (:Started
    (bind _closed (Public|HUD|CloseLastActiveWidget))
    (if (not _closed)
      (bind _isoppened (Public|HUD|ChangeWidgetState (Variables|UIClasses|GetPauseMenuClass)))
      (bind _output_get (Variables|UIClasses|SetPauseMenuIsActive _isoppened))
      (Game|SetGamePaused _output_get))))

(event Input|EnhancedActionEvents|EnhancedInputActionINPA_PlayerMenu
  (params (ActionValue :type Boolean) (ElapsedSeconds :type Float%20%28double-precision%29) (TriggeredSeconds :type Float%20%28double-precision%29) (InputAction :type Input%20Action%20Object%20Reference :default "/Game/Main/Inputs/INPA_PlayerMenu.INPA_PlayerMenu"))
  ;[1 1 1] Инпуты меню
  (:Started
    (if (not (Variables|UIClasses|GetPauseMenuIsActive))
      (Public|HUD|ChangeWidgetState (Variables|UIClasses|GetPlayerMenuClasses)))))

(event Input|EnhancedActionEvents|EnhancedInputActionINPA_Interact
  (params (ActionValue :type Boolean) (ElapsedSeconds :type Float%20%28double-precision%29) (TriggeredSeconds :type Float%20%28double-precision%29) (InputAction :type Input%20Action%20Object%20Reference :default "/Game/Main/Inputs/INPA_Interact.INPA_Interact"))
  ;[1 1 1] Взаимодействие с предметами
  (bind _playerpawn (Variables|Other|GetPlayerPawn)
    (:then
      (Default|TryInteractItem _playerpawn))
    (:else)))

(event EventBeginPlay
  ;[1 1 1] Event BeginPlay
  (|CallParentFunction)
  (Protected|InitVariables)
  (Protected|BindingEvents))

(fn ConstructionScript)

(fn WidgetIsOpennedbyClass
  (params (Class :type UI%20Full%20Screen%20Widget%20Class%20Reference))
  (LocalVariables|SetL_Class Class)
  (for _array_element (Variables|Other|GetOppenedWidgets)
    (bind _output_get (LocalVariables|SetL_Widget _array_element))
    (if (== (Utilities|GetClass _output_get) (LocalVariables|GetL_Class))
      (return true)))
  (return false))

(fn CloseFullScreenWidgetbyClass
  (params (Class :type UI%20Full%20Screen%20Widget%20Class%20Reference))
  (LocalVariables|SetL_Class Class)
  (for _array_element (Variables|Other|GetOppenedWidgets)
    (bind _output_get (LocalVariables|SetL_Widget _array_element))
    (if (== (Utilities|GetClass _output_get) (LocalVariables|GetL_Class))
      (Public|HUD|CloseFullScreenWidget (LocalVariables|GetL_Widget)))))

(fn CloseFullScreenWidget
  (params (Wigdet :type UI%20Full%20Screen%20Widget%20Object%20Reference))
  (bind _output_get (LocalVariables|SetL_Widget Wigdet))
  (Utilities|IsValid _output_get
    (:Is%20Valid
      (Utilities|Array|RemoveItem (Variables|Other|GetOppenedWidgets) (LocalVariables|GetL_Widget))
      (Widget|RemovefromParent (LocalVariables|GetL_Widget))
      (for _array_element (Variables|Other|GetOppenedWidgets)
        (if (Default|GetIsActiveWidget _array_element)
          (return)))
      (Variables|Default|SetbShowMouseCursor false)
      (Input|SetInputModeGameOnly self false)
      (Public|HUD|EnableControllerInputs true))))

(fn OpenFullScreenWidgetbyClass
  (params (Class :type UI%20Full%20Screen%20Widget%20Class%20Reference))
  (bind _returnvalue (UserInterface|CreateWidget Class))
  (Public|HUD|OpenFullScreenWidget _returnvalue)
  (return _returnvalue))

(fn OpenFullScreenWidget
  (params (Widget :type UI%20Full%20Screen%20Widget%20Object%20Reference))
  (bind _output_get (LocalVariables|SetL_Widget Widget))
  (LocalVariables|SetL_Active (Default|GetIsActiveWidget _output_get))
  (Variables|Other|GetHUD_UI
    (:then
      (Utilities|FlowControl|Sequence
        (:then_0
          (Utilities|FlowControl|Sequence
            (:then_0
              (if (not (UserInterface|Viewport|IsinViewport (LocalVariables|GetL_Widget)))
                (Default|AddFullscreenWidget (Variables|Other|GetHUD_UI) (LocalVariables|GetL_Widget) (LocalVariables|GetL_Active))))
            (:then_1
              (if (LocalVariables|GetL_Active)
                (Input|SetInputModeGameandUI self 0 "DoNotLock" false false)
                (Variables|Default|SetbShowMouseCursor true)
                (Public|HUD|EnableControllerInputs false)))))
        (:then_1
          (Utilities|Array|Add (Variables|Other|GetOppenedWidgets) (LocalVariables|GetL_Widget)))))
    (:else)))

(fn InitBaseHUD
  (Public|HUD|OpenFullScreenWidgetbyClass "/Game/Main/Blueprints/UI/UI_PlayerHUD.UI_PlayerHUD_C"))

(fn InitInputs
  (Input|AddMappingContext (PlayerController|LocalPlayerSubsystems|GetEnhancedInputLocalPlayerSubsystem self) "/Game/Main/Inputs/INPC_Menu.INPC_Menu" 0 "(bIgnoreAllPressedKeysUntilRelease=True,bForceImmediately=False,bNotifyUserSettings=False)")
  (Public|HUD|EnableControllerInputs true))

(fn InitVariables
  (bind _asbp_basic_hud (Utilities|Casting|CastToBP_BasicHUD (HUD|GetHUD)))
  (Variables|Other|SetHUDObject _asbp_basic_hud)
  (bind _asbp_playable_character_base (Utilities|Casting|CastToBP_PlayableCharacterBase (Game|Player|GetPlayerPawn 0)))
  (Variables|Other|SetPlayerPawn _asbp_playable_character_base)
  (Protected|InitInputs))

(fn BindonHUDInit
  (Variables|Other|SetHUD_UI (Default|GetHUD (Variables|Other|GetHUDObject)))
  (Protected|HUD|InitBaseHUD))

(fn BindingEvents
  (EventDispatchers|BindEventtoOnHudInit (Variables|Other|GetHUDObject) (EventDispatchers|CreateEvent :!event BindonHUDInit)))

(fn ChangeWidgetState
  (params (Class :type UI%20Full%20Screen%20Widget%20Class%20Reference))
  (bind _output_get (LocalVariables|SetL_Class Class))
  (if (Public|HUD|Get|WidgetIsOpennedbyClass _output_get)
    (Public|HUD|CloseFullScreenWidgetbyClass (LocalVariables|GetL_Class))
    (return false 0)
    (else
      (bind _returnvalue (Public|HUD|OpenFullScreenWidgetbyClass (LocalVariables|GetL_Class)))
      (return true _returnvalue))))

(fn CloseLastActiveWidget
  (bind _arrayelement (Utilities|Array|ReverseforEachLoop (Variables|Other|GetOppenedWidgets))
    (:LoopBody
      (if (Default|GetIsActiveWidget _arrayelement)
        (Public|HUD|CloseFullScreenWidget _arrayelement)
        (return true)))
    (:Completed
      (return false))))

(fn EnableControllerInputs
  (params (Enable :type Boolean))
  (if Enable
    (Input|AddMappingContext (PlayerController|LocalPlayerSubsystems|GetEnhancedInputLocalPlayerSubsystem self) "/Game/Main/Inputs/INPC_Move.INPC_Move" 0 "(bIgnoreAllPressedKeysUntilRelease=True,bForceImmediately=False,bNotifyUserSettings=False)")
    (Input|AddMappingContext (PlayerController|LocalPlayerSubsystems|GetEnhancedInputLocalPlayerSubsystem self) "/Game/Main/Inputs/INPC_Mouse.INPC_Mouse" 0 "(bIgnoreAllPressedKeysUntilRelease=True,bForceImmediately=False,bNotifyUserSettings=False)")
    (Input|AddMappingContext (PlayerController|LocalPlayerSubsystems|GetEnhancedInputLocalPlayerSubsystem self) "/Game/Main/Inputs/INPC_View.INPC_View" 0 "(bIgnoreAllPressedKeysUntilRelease=True,bForceImmediately=False,bNotifyUserSettings=False)")
    (Input|AddMappingContext (PlayerController|LocalPlayerSubsystems|GetEnhancedInputLocalPlayerSubsystem self) "/Game/Main/Inputs/INPC_HUDInGame.INPC_HUDInGame" 0 "(bIgnoreAllPressedKeysUntilRelease=True,bForceImmediately=False,bNotifyUserSettings=False)")
    (else
      (Input|RemoveMappingContext (PlayerController|LocalPlayerSubsystems|GetEnhancedInputLocalPlayerSubsystem self) "/Game/Main/Inputs/INPC_Move.INPC_Move" "(bIgnoreAllPressedKeysUntilRelease=True,bForceImmediately=False,bNotifyUserSettings=False)")
      (Input|RemoveMappingContext (PlayerController|LocalPlayerSubsystems|GetEnhancedInputLocalPlayerSubsystem self) "/Game/Main/Inputs/INPC_Mouse.INPC_Mouse" "(bIgnoreAllPressedKeysUntilRelease=True,bForceImmediately=False,bNotifyUserSettings=False)")
      (Input|RemoveMappingContext (PlayerController|LocalPlayerSubsystems|GetEnhancedInputLocalPlayerSubsystem self) "/Game/Main/Inputs/INPC_View.INPC_View" "(bIgnoreAllPressedKeysUntilRelease=True,bForceImmediately=False,bNotifyUserSettings=False)")
      (Input|RemoveMappingContext (PlayerController|LocalPlayerSubsystems|GetEnhancedInputLocalPlayerSubsystem self) "/Game/Main/Inputs/INPC_HUDInGame.INPC_HUDInGame" "(bIgnoreAllPressedKeysUntilRelease=True,bForceImmediately=False,bNotifyUserSettings=False)"))))